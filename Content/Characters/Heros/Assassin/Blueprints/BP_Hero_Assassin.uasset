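; Assassin hero Blueprint that implements a normal attack and a teleport-strike skill, building on inherited hero helpers.
; Both attacks play montages with input disabled until completion.
; The skill sphere-traces forward, teleports to each hit actor failing the camp check, adjusts rotation, and doubles default damage until its montage completes.
; Separate hurt events run their own sphere traces and pass hits to a shared detection function to apply damage.
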(event `self.ReceiveBeginPlay`
  (`parent.ReceiveBeginPlay`))

(event `self.CE_ExecuteNormalAttak`
  ;[1 1 1] 普通攻击
  (`self.DisableInput` null)
  (`|PlayMontage` (`self.Mesh`) "/Game/Characters/Heros/Assassin/Animations/Attack_C_Montage.Attack_C_Montage"
    (:`OnCompleted`
      (`self.EnableInput` null))))

(event `self.CE_ExecuteSkillAttak`
  ;[1 1 1] 技能攻击
  (bind _outhits (`self.FUN_Forward_MultiSpereTraceForObjects` 300.0 200.0 300.0 self))
  (for _array_element _outhits
    (bind (_bblockinghit _binitialoverlap _time _distance _location _impactpoint _normal _impactnormal _physmat _hitactor) (`GameplayStatics.BreakHitResult` _array_element))
    (bind _output_get (`self.FUN_CampCheckForObjects` _hitactor))
    (if (not _output_get)
      (`self.DisableInput` null)
      (set `self.CurrentDamage` (* 2 (`.DefaultDamge_19_FEFDC9F547540E607FBA77B1D193316C` (break `/Game/Characters/Heros/F_HeroAttribute` (`self.HeroAttribute`)))))
      (`self.K2_TeleportTo` (`self.K2_GetActorLocation` _hitactor) (`self.K2_GetActorRotation`))
      (`self.FUN_SetActorRotation`)
      (`|PlayMontage` (`self.Mesh`) "/Game/Characters/Heros/Assassin/Animations/Attack_E_SetB_Montage.Attack_E_SetB_Montage"
        (:`OnCompleted`
          (set `self.CurrentDamage` (`.DefaultDamge_19_FEFDC9F547540E607FBA77B1D193316C` (break `/Game/Characters/Heros/F_HeroAttribute` (`self.HeroAttribute`))))
          (`self.EnableInput` null))))))

(event `self.CE_MakeNormalHurt`
  ;[1 1 1] 检测普通攻击击中对象并应用伤害
  (bind (_outhits _returnvalue) (`self.FUN_Forward_MultiSpereTraceForObjects` 80.0 90.0 150.0 self))
  (`self.FUN_DetectionAttackTarget` _outhits _returnvalue))

(event `self.CE_MakeSkillHurt`
  ;[1 1 1] 检测技能攻击击中对象并应用伤害
  (bind (_outhits _returnvalue) (`self.FUN_Forward_MultiSpereTraceForObjects` 160.0 0.0 0.0 self))
  (`self.FUN_DetectionAttackTarget` _outhits _returnvalue))

(fn `UserConstructionScript`
  (`parent.UserConstructionScript`))