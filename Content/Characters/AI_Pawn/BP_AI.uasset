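; BP_AI is an AI pawn that takes damage and destroys itself when its health runs out.
; AnyDamage calls the CEServerReplicateHurt event, which is empty here, and subtracts the damage from CurrentHealth.
; At zero health it resets AINumber on BPAIBuilder to zero, then destroys its capsule, mesh and actor.
; The construction script runs the parent's and assigns the pawn to camp index 1.
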(event `self.ReceiveBeginPlay`
  (`parent.ReceiveBeginPlay`))

(event `self.CE_Server_ReplicateHurt`)

(event `self.ReceiveAnyDamage`
  (params (Damage :type "Float (single-precision)") (DamageType :type "DamageType Object Reference") (InstigatedBy :type "Controller Object Reference") (DamageCauser :type "Actor Object Reference"))
  (`self.CE_Server_ReplicateHurt`)
  (bind _output_get (set `self.CurrentHealth` (- (`self.CurrentHealth`) Damage)))
  (if (<= _output_get 0.0)
    (set `self.CurrentHealth` 0.0)
    (set `/Game/SceneModules/Item/BP_AI_Builder.AI_Number` 0 (`self.BP_AI_Builder`))
    (`ActorComponent.K2_DestroyComponent` (`self.CapsuleComponent`))
    (`ActorComponent.K2_DestroyComponent` (`self.Mesh`))
    (`self.K2_DestroyActor`)))

(fn `UserConstructionScript`
  (`parent.UserConstructionScript`)
  (set `self.Player Camp Index` 1))