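; BP_LobbyCamera is a lobby actor that spawns and manages a player's displayed hero on the server.
; The construction script caches DT_HeroAttribute row names, letting hero switches replace the default Tank by index.
; Heroes spawn at the Scene component with player name and ID, and are destroyed on EndPlay.
; A RepNotify copies camp index to the hero, while a separate event updates HP color.
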(event `self.ReceiveBeginPlay`)

(event `EVE_SpawnHero`
  ;[1 1 1] 生成默认Hero【服务器执行事件】
  (bind _returnvalue (`|GetDataTableRow` "/Game/Characters/Heros/DT_HeroAttribute.DT_HeroAttribute" "Tank")
    (:`then`
      (`self.FUN_SpawnHero` (`.HeroType_2_F41A0DA2484FBBF976B9B98DCF4E3E16` (break `/Game/Characters/Heros/F_HeroAttribute` _returnvalue))))))

(event `EVE_Update_HeroType`
  (params (HeroIndex :type Integer))
  ;[1 1 1] 根据客户端或服务器的 UMG 切换 HeroIndex 在服务器上切换 HeroType 【服务器执行事件】
  (set `self.HeroIndex` HeroIndex)
  (`self.K2_DestroyActor` (`self.CurrentHero`))
  (bind _returnvalue (`|GetDataTableRow` "/Game/Characters/Heros/DT_HeroAttribute.DT_HeroAttribute" (`|GetArrayItem` (`self.Out Row Names`) HeroIndex))
    (:`then`
      (`self.FUN_SpawnHero` (`.HeroType_2_F41A0DA2484FBBF976B9B98DCF4E3E16` (break `/Game/Characters/Heros/F_HeroAttribute` _returnvalue))))))

(event `EVE_Set_CampIndex`
  (params (PlayerCampIndex :type Integer))
  ;[1 1 1] 设置阵营索引
  (set `self.PlayerCampIndex` PlayerCampIndex))

(event `self.ReceiveEndPlay`
  (params (EndPlayReason :type "EEndPlayReason Enum" :default "Destroyed"))
  (bind _currenthero (`self.CurrentHero`))
  ;[1 1 1] 客户端退出 session 时销毁在服务器上创建的 Pawn
  (`/Engine/EditorBlueprintResources/StandardMacros.IsValid` _currenthero
    (:`Is Valid`
      (`self.K2_DestroyActor` _currenthero))))

(event `EVE_UpadatePlayerCamp`
  (params (`目标` :type "/Game/UMGs/UMG_Characters/UMG_Player_HP Object Reference"))
  ;[1 1 1] 根据阵营切换 HP Color
  (`/Engine/EditorBlueprintResources/StandardMacros.IsValid` `目标`
    (:`Is Valid`
      (`/Game/UMGs/UMG_Characters/UMG_Player_HP.Update HP Color` `目标` (`self.PlayerCampIndex`)))))

(fn `FUN_SpawnHero`
  (params (Class :type "/Game/Characters/Heros/Base/Blueprint/BP_Hero_Base Class Reference"))
  (bind _returnvalue (`|SpawnActorFromClass` Class (`SceneComponent.K2_GetComponentToWorld` (`self.Scene`)) "Undefined" "OverrideRootScale" null (`self.PlayerName`) (`self.PlayerID`) 0 null))
  (set `self.CurrentHero` _returnvalue)
  (bind _output_get (set `self.As BP Hero Base` _returnvalue))
  (`/Game/Characters/Heros/Base/Blueprint/BP_Hero_Base.FUN_Upadte PlayerName` _output_get))

(fn `OnRep_PlayerCampIndex`
  (bind _as_bp_hero_base (`self.As BP Hero Base`))
  (`/Engine/EditorBlueprintResources/StandardMacros.IsValid` _as_bp_hero_base
    (:`Is Valid`
      (set `/Game/Characters/Heros/Base/Blueprint/BP_Hero_Base.Player Camp Index` (`self.PlayerCampIndex`) _as_bp_hero_base))))

(fn `UserConstructionScript`
  (bind _outrownames (`DataTableFunctionLibrary.GetDataTableRowNames` "/Game/Characters/Heros/DT_HeroAttribute.DT_HeroAttribute"))
  (set `self.Out Row Names` _outrownames))