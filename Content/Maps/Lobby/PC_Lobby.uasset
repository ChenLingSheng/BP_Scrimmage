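; Lobby PlayerController that creates the lobby UI, spawns each player's BP_LobbyCamera pawn and bridges lobby state between server and clients.
; On local BeginPlay it passes the GameInstance name to a server event, which spawns and possesses the pawn at an indexed PlayerStart.
; The server then pushes all names and IDs to every controller's UI.
; Other events handle game mode, camp assignment, loading screen and leaving the session.
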(event `self.ReceiveBeginPlay`
  ;[1 1 1] 生成UMG及调用生成PlayerPawn
  ;;[1 1 1] 只在本地执行
  (if (`self.IsLocalPlayerController`)
    (`self.FUN_Create_UMG_Lobby`)
    (set `self.bShowMouseCursor` true)
    (bind _asgi_main (cast `/Game/GI_Main` (`GameplayStatics.GetGameInstance`)))
    (`self.CE_Spawn_Player` (`/Game/GI_Main.PlayerName` _asgi_main))))

(event `CE_Spawn_Player`
  (params (PlayerName :type Text))
  (bind (_returnvalue_year _returnvalue_month _returnvalue_day _returnvalue_hour _returnvalue_minute _returnvalue_second _returnvalue_millisecond) (`KismetMathLibrary.BreakDateTime` (`KismetMathLibrary.Now`)))
  ;[1 1 1] 调用在服务器上运行的生成PlayerPawn
  (bind _asgm_lobby (cast `/Game/Maps/Lobby/GM_Lobby` (`GameplayStatics.GetGameMode`)))
  (bind _outactors (`GameplayStatics.GetAllActorsOfClass` "/Script/Engine.PlayerStart"))
  (bind _returnvalue (`|SpawnActorFromClass` "/Game/Maps/Lobby/BP_LobbyCamera.BP_LobbyCamera_C" (`self.GetTransform` (`|GetArrayItem` _outactors (`/Game/Maps/Lobby/GM_Lobby.PC_ListIndex` _asgm_lobby))) "Undefined" "OverrideRootScale" null PlayerName (`KismetStringLibrary.Concat_StrStr` (`KismetStringLibrary.Conv_IntToString` _returnvalue_year) (`KismetStringLibrary.Conv_IntToString` _returnvalue_month) (`KismetStringLibrary.Conv_IntToString` _returnvalue_day) (`KismetStringLibrary.Conv_IntToString` _returnvalue_hour) (`KismetStringLibrary.Conv_IntToString` _returnvalue_minute) (`KismetStringLibrary.Conv_IntToString` _returnvalue_second) (`KismetStringLibrary.Conv_IntToString` _returnvalue_millisecond)) 0 null))
  (`self.Possess` self _returnvalue)
  (`/Game/Maps/Lobby/BP_LobbyCamera.EVE_SpawnHero` _returnvalue)
  (`self.FUN_Update_PlayerList`))

(event `CE_Client_Update_PlayerList`
  (params (PlayerName :type "Array of Text (by ref)") (PlayerID :type "Array of String (by ref)"))
  ;[1 1 1] 更新玩家列表【客户端】
  (`/Game/UMGs/UMG_Lobbys/UMG_Lobby.FUN_UpdatePlayer` (`self.UMG_Lobby`) PlayerName PlayerID))

(event `CE_Update_Map`
  (params (`游戏模式索引` :type Integer))
  ;[1 1 1] 更新游戏模式
  (bind _asgs_lobby (cast `/Game/Maps/Lobby/GS_Lobby` (`GameplayStatics.GetGameState`)))
  (set `/Game/Maps/Lobby/GS_Lobby.游戏模式索引` `游戏模式索引` _asgs_lobby))

(event `CE_Client_Quit_Session`
  ;[1 1 1] 退出房间
  (`DestroySessionCallbackProxy.DestroySession` self
    (:`OnSuccess`
      (`GameplayStatics.OpenLevelBySoftObjectPtr` "/Game/Maps/Login/L_Login.L_Login"))))

(event `CE_Client_Loding`
  ;[1 1 1] 进入加载界面【本地客户端/服务端】
  (bind _returnvalue (`|CreateWidget` "/Game/UMGs/UMG_Loading.UMG_Loading_C" self))
  (`UserWidget.AddToViewport` _returnvalue 10))

(event `CE_GetPlayerIndex`
  (params (PlayerIndex :type Integer))
  ;[1 1 1] 从服务端获取玩家在所在阵营中的索引号
  (bind _asgi_main (cast `/Game/GI_Main` (`GameplayStatics.GetGameInstance`)))
  (bind _result (`/Engine/EditorBlueprintResources/StandardMacros.DecrementInt` PlayerIndex)
    (:`  `
      (set `/Game/GI_Main.playerIndexForCamp` _result _asgi_main))))

(event `CE_ResetPlayerCampIndex`
  (params (PlayerCampIndex :type Integer))
  ;[1 1 1] 游戏开始时，若所有玩家的阵营都是相同的，则服务端随机选择一个玩家的 PC_Lobby 调用此事件，强制修改其阵营为其余玩家阵营为对立阵营
  (bind _asgi_main (cast `/Game/GI_Main` (`GameplayStatics.GetGameInstance`)))
  (set `/Game/GI_Main.PlayerCampIndex` PlayerCampIndex _asgi_main)
  (set `/Game/GI_Main.playerIndexForCamp` 0 _asgi_main))

(event `CE_GetPlayerCampIndex`
  ;[1 1 1] 获取玩家当前阵营索引
  (bind _asbp_lobby_camera (cast `/Game/Maps/Lobby/BP_LobbyCamera` (`GameplayStatics.GetPlayerPawn` 0)))
  (set `self.PlayerCampIndex` (`/Game/Maps/Lobby/BP_LobbyCamera.PlayerCampIndex` _asbp_lobby_camera)))

(fn `FUN_Create_UMG_Lobby`
  (bind _returnvalue (`|CreateWidget` "/Game/UMGs/UMG_Lobbys/UMG_Lobby.UMG_Lobby_C" self))
  (set `self.UMG_Lobby` _returnvalue)
  (`UserWidget.AddToViewport` _returnvalue 0))

(fn `FUN_Update_PlayerList`
  (locals (Names :type "Array of Text") (IDs :type "Array of String"))
  (for _array_element (`/Game/Maps/Lobby/GM_Lobby.PC_List` (cast `/Game/Maps/Lobby/GM_Lobby` (`GameplayStatics.GetGameMode`) :!pure true))
    (bind _asbp_lobby_camera (cast `/Game/Maps/Lobby/BP_LobbyCamera` (`self.K2_GetPawn` _array_element)))
    (`KismetArrayLibrary.Array_Add` (`local.Names`) (`/Game/Maps/Lobby/BP_LobbyCamera.PlayerName` _asbp_lobby_camera))
    (`KismetArrayLibrary.Array_Add` (`local.IDs`) (`/Game/Maps/Lobby/BP_LobbyCamera.PlayerID` _asbp_lobby_camera)))
  ;[1 1 1] 在客户端上调用自己拥有的玩家控制器来更新玩家列表
  (for _array_element_2 (`/Game/Maps/Lobby/GM_Lobby.PC_List` (cast `/Game/Maps/Lobby/GM_Lobby` (`GameplayStatics.GetGameMode`) :!pure true))
    (`self.CE_Client_Update_PlayerList` _array_element_2 (`local.Names`) (`local.IDs`))))

(fn `UserConstructionScript`)