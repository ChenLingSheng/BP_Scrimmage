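; BP_RecoverHealth is a pickup item that restores a fixed amount of health to the actor that picks it up.
; It implements the PickUpItemResult event, adding the amount to that actor's CurrentHealth and clamping the result to the MaxHealth in its HeroAttribute.
; The default BeginPlay, overlap and Tick events are disabled placeholders, and the construction script only calls its parent.
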(event `self.PickUpItemResult`
  (params (`Other Actor` :type "/Game/Characters/Heros/Base/Blueprint/BP_Hero_Base Object Reference"))
  (bind _currenthealth (`/Game/Characters/Heros/Base/Blueprint/BP_Hero_Base.CurrentHealth` `Other Actor`))
  (bind ((`MaxHealth_5_E28E13AE4B6443E577ABDCBFC5B5837F` _maxhealth)) (break `/Game/Characters/Heros/F_HeroAttribute` (`/Game/Characters/Heros/Base/Blueprint/BP_Hero_Base.HeroAttribute` `Other Actor`)))
  (set `/Game/Characters/Heros/Base/Blueprint/BP_Hero_Base.CurrentHealth` (+ _currenthealth 500.0) `Other Actor`)
  (if (>= _currenthealth _maxhealth)
    (set `/Game/Characters/Heros/Base/Blueprint/BP_Hero_Base.CurrentHealth` _maxhealth `Other Actor`)))

(fn `UserConstructionScript`
  (`parent.UserConstructionScript`))