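; BP_ShooterBullet_Skill is the Shooter hero's ranged skill bullet, with custom hit responses for characters and breakable scenery.
; On hitting an enemy character, it nudges the target along the bullet's horizontal forward vector and doubles its own Damage variable, without destroying itself.
; On hitting a breakable, it calls that object's CEDestroyActor event and destroys itself.
; Hit detection and damage application are not in this graph, and its BeginPlay, Overlap and Tick events are disabled.
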(event `self.CE_AttackPlayer`
  (params (NewParam :type "Actor Object Reference"))
  (bind (_returnvalue_x _returnvalue_y) (`KismetMathLibrary.BreakVector` (`self.GetActorForwardVector`)))
  ;[1 1 1] 对敌方角色造成击退效果
  (`/Engine/EditorBlueprintResources/StandardMacros.IsValid` NewParam
    (:`Is Valid`
      (`self.K2_AddActorWorldOffset` NewParam (`KismetMathLibrary.MakeVector` (* 20 _returnvalue_x) (* 20 _returnvalue_y)) false false)
      (set `self.Damage` (* 2 (`self.Damage`))))))

(event `self.CE_AttackBreakable`
  (params (NewParam :type "/Game/SceneModules/Terrains/Breakable/BP_Breakable_Base Object Reference"))
  ;[1 1 1] 子弹击中可破坏场景构件，调用场景构件自身销毁事件，同时销毁子弹自身
  (`/Game/SceneModules/Terrains/Breakable/BP_Breakable_Base.CE_Destroy_Actor` NewParam)
  (`self.K2_DestroyActor`))

(fn `UserConstructionScript`)