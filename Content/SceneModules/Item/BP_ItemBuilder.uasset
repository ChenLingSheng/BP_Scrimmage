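; Item spawner actor that places a health recovery pickup at its own location and respawns it after it is taken.
; On BeginPlay it spawns the item and hands it a reference back to the builder.
; A one-second Delay loop polls ItemNumber; when it reaches zero, a one-shot 20-second timer re-enters the spawn logic.
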(event `self.ReceiveBeginPlay`
  ;[1 1 1] 生成指定物品，且每两秒检测一次当前物品是否被拾取，若物品已经被拾取则在20秒后重新生成指定物品
  (bind _returnvalue (`|SpawnActorFromClass` "/Game/SceneModules/Item/RecoverHealth/BP_RecoverHealth.BP_RecoverHealth_C" (`KismetMathLibrary.MakeTransform` (`self.K2_GetActorLocation` self) (`self.K2_GetActorRotation` self)) "Undefined" "OverrideRootScale" null null :!label _label))
  (set `/Game/SceneModules/Item/BP_ItemBase.BP_ItemBuilder` self _returnvalue)
  (set `self.ItemNumber` 1)
  (if (== (`self.ItemNumber`) 0) :!label _label_2
    (`KismetSystemLibrary.K2_SetTimerDelegate` (delegate `RebuildItem`) 20.0)
    (else
      (`KismetSystemLibrary.Delay` 1.0)
      (goto _label_2))))

(event `RebuildItem`
  ;[1 1 1] 生成指定物品，且每两秒检测一次当前物品是否被拾取，若物品已经被拾取则在20秒后重新生成指定物品
  (goto _label))

(fn `UserConstructionScript`)