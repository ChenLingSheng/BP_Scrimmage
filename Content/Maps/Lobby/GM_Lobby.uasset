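; GM_Lobby is the lobby game mode that tracks joined players and launches the match.
; Login and logout maintain an array of PC_Lobby controllers, with logout refreshing the first controller's player list, and a lookup finds controllers by their camera pawn's ID.
; Starting numbers players within two camps, moving the last player if one camp is empty.
; It then triggers client loading and, after a delay, runs ServerTravel to the selected map.
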(event `self.ReceiveBeginPlay`)

(event `self.K2_PostLogin`
  (params (NewPlayer :type "PlayerController Object Reference"))
  ;[1 1 1] 玩家加入：将进入大厅的新玩家的控制器添加到数组中
  (bind _aspc_lobby (cast `/Game/Maps/Lobby/PC_Lobby` NewPlayer))
  (bind _returnvalue (`KismetArrayLibrary.Array_AddUnique` (`self.PC_List`) _aspc_lobby))
  (set `self.PC_ListIndex` _returnvalue))

(event `self.K2_OnLogout`
  (params (ExitingController :type "Controller Object Reference"))
  ;[1 1 1] 玩家退出：将退出大厅的玩家的控制器从数组中移除
  (bind _aspc_lobby (cast `/Game/Maps/Lobby/PC_Lobby` ExitingController))
  (`KismetArrayLibrary.Array_RemoveItem` (`self.PC_List`) _aspc_lobby)
  ;[1 1 1] 更新玩家列表
  (bind _aspc_lobby_2 (cast `/Game/Maps/Lobby/PC_Lobby` (`GameplayStatics.GetPlayerController` 0)))
  (`/Game/Maps/Lobby/PC_Lobby.FUN_Update_PlayerList` _aspc_lobby_2))

(event `CE_StartGame`
  (params (GameMapIndex :type Integer))
  ;[1 1 1] 开始游戏（服务器特有，在UMG_Lobby中调用）
  (`self.CE_SetCampNumberFoPlayer`)
  (`self.CE_SwitchToTheTargetMap` GameMapIndex))

(event `CE_SetCampNumberFoPlayer`
  ;[1 1 1] 设置两个对立阵营人数
  (for _array_element (`self.PC_List`)
    (`self.CE_RecordCampPlayerIndex` _array_element))
  (`self.ResetPlayerCamp`))

(event `CE_RecordCampPlayerIndex`
  (params (PC_Lobby :type "/Game/Maps/Lobby/PC_Lobby Object Reference"))
  ;[1 1 1] 记录玩家所在阵营中的序列号
  (`/Game/Maps/Lobby/PC_Lobby.CE_GetPlayerCampIndex` PC_Lobby)
  (if (== (`/Game/Maps/Lobby/PC_Lobby.PlayerCampIndex` PC_Lobby) 0)
    (bind _result (`/Engine/EditorBlueprintResources/StandardMacros.IncrementInt` (`self.CampA_playerNumber`))
      (:`  `
        (bind _output_get (set `self.CampA_playerNumber` _result))
        (`/Game/Maps/Lobby/PC_Lobby.CE_GetPlayerIndex` PC_Lobby _output_get)))
    (else
      (bind _result_2 (`/Engine/EditorBlueprintResources/StandardMacros.IncrementInt` (`self.CampB_playerNumber`))
        (:`  `
          (bind _output_get_2 (set `self.CampB_playerNumber` _result_2))
          (`/Game/Maps/Lobby/PC_Lobby.CE_GetPlayerIndex` PC_Lobby _output_get_2))))))

(event `CE_SwitchToTheTargetMap`
  (params (GameMapIndex :type Integer))
  ;[1 1 1] 正进入房主选定的游戏地图
  (for _array_element (`self.PC_List`)
    (`/Game/Maps/Lobby/PC_Lobby.CE_Client_Loding` _array_element))
  (`KismetSystemLibrary.Delay` 1.0)
  (`KismetSystemLibrary.ExecuteConsoleCommand` (`KismetStringLibrary.Concat_StrStr` "ServerTravel " (select `int` GameMapIndex :`0` "L_VaultDefend" :`1` "L_CapturePlace" :`2` "")) (`GameplayStatics.GetPlayerController` 0)))

(fn `FUN_Find_PC_ByID`
  (params (ID :type String))
  (returns (PC :type "/Game/Maps/Lobby/PC_Lobby Object Reference"))
  (for _array_element (`self.PC_List`)
    (bind _asbp_lobby_camera (cast `/Game/Maps/Lobby/BP_LobbyCamera` (`Controller.K2_GetPawn` _array_element)))
    (if (`KismetStringLibrary.EqualEqual_StrStr` (`/Game/Maps/Lobby/BP_LobbyCamera.PlayerID` _asbp_lobby_camera) ID)
      (return _array_element))))

(fn `ResetPlayerCamp`
  (bind _pc_list (`self.PC_List`))
  ;[1 1 1] 当所有玩家都为同一阵营时，选择玩家列表的最后一位玩家重新设置其阵营使得游戏开始时形成两个对立阵营
  (if (< (`KismetArrayLibrary.Array_Length` (`self.PC_List`)) 2)
    _
    (elif (== 0 (`self.CampA_playerNumber`))
      (set `self.PlayerCampIndex` 0)
      (`/Game/Maps/Lobby/PC_Lobby.CE_ResetPlayerCampIndex` (`|GetArrayItem` _pc_list (- (`KismetArrayLibrary.Array_Length` _pc_list) 1)) (`self.PlayerCampIndex`) :!label _label)
      (elif (== 0 (`self.CampB_playerNumber`))
        (set `self.PlayerCampIndex` 1)
        (goto _label)
        (else
          _))))
  (return))

(fn `UserConstructionScript`)