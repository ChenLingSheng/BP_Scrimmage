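; BP_Death_Camera is a controllable character pawn, named as the hero death camera, that the player moves with axis input.
; MoveForward and MoveRight feed movement input to the CharacterMovement component's owning pawn along the control rotation's forward and right vectors.
; The forward vector uses the full control rotation, so it follows view pitch as well as yaw.
; The graph holds no look, death or camera-switching logic.
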(event `InputAxis|MoveForward`
  (params (AxisValue :type "Float (single-precision)"))
  (bind _returnvalue (`PawnMovementComponent.GetPawnOwner` (`self.CharacterMovement`)))
  ;[1 1 1] Move
  (`self.AddMovementInput` _returnvalue (`KismetMathLibrary.GetForwardVector` (`self.GetControlRotation` _returnvalue)) AxisValue false))

(event `InputAxis|MoveRight`
  (params (AxisValue :type "Float (single-precision)"))
  (bind _returnvalue (`PawnMovementComponent.GetPawnOwner` (`self.CharacterMovement`)))
  ;[1 1 1] Move
  (`self.AddMovementInput` _returnvalue (`KismetMathLibrary.GetRightVector` (`self.GetControlRotation` _returnvalue)) AxisValue false))

(fn `UserConstructionScript`)