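; Player controller for the practice room map that lets the player switch between heroes in place.
; On begin play it shows the practice room widget and the mouse cursor.
; Pressing Q briefly delays, cycles the hero index stored in GI_Main, then looks up the hero class in DT_HeroAttribute.
; It spawns that hero at the current pawn's transform, destroys the old pawn, possesses the new one and resets controller rotation.
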(event `self.ReceiveBeginPlay`
  (`parent.ReceiveBeginPlay`)
  (bind _returnvalue (`|CreateWidget` "/Game/UMGs/UMG_PracticeRoom.UMG_PracticeRoom_C" self))
  (`UserWidget.AddToViewport` _returnvalue 0)
  (set `self.bShowMouseCursor` true))

(event `Key|Q`
  (params (Key :type "Key Structure"))
  ;[1 1 1] 切换英雄角色
  (:`Pressed`
    (`KismetSystemLibrary.Delay` 0.2)
    (bind _asgi_main (cast `/Game/GI_Main` (`GameplayStatics.GetGameInstance`)))
    (bind _playerheroindex (`/Game/GI_Main.PlayerHeroIndex` _asgi_main))
    (if (< _playerheroindex 2)
      (bind _result (`/Engine/EditorBlueprintResources/StandardMacros.IncrementInt` _playerheroindex)
        (:`  `
          (set `/Game/GI_Main.PlayerHeroIndex` _result _asgi_main)))
      (else
        (set `/Game/GI_Main.PlayerHeroIndex` 0 _asgi_main)))
    (`self.SpawnHero`)))

(event `SpawnHero`
  (bind _returnvalue (`GameplayStatics.GetPlayerPawn` 0))
  ;[1 1 1] 生成新角色
  (bind _asgi_main (cast `/Game/GI_Main` (`GameplayStatics.GetGameInstance`)))
  (bind _returnvalue_2 (`|GetDataTableRow` "/Game/Characters/Heros/DT_HeroAttribute.DT_HeroAttribute" (`|GetArrayItem` (`self.HeroNames`) (`/Game/GI_Main.PlayerHeroIndex` _asgi_main)))
    (:`then`
      (bind _returnvalue_3 (`|SpawnActorFromClass` (`.HeroType_2_F41A0DA2484FBBF976B9B98DCF4E3E16` (break `/Game/Characters/Heros/F_HeroAttribute` _returnvalue_2)) (`KismetMathLibrary.MakeTransform` (`self.K2_GetActorLocation` _returnvalue) (`self.K2_GetActorRotation` _returnvalue)) "Undefined" "OverrideRootScale" null (`/Game/GI_Main.PlayerName` _asgi_main) "" 0 null))
      ;[1 1 1] 销毁原有Pawn
      (`self.K2_DestroyActor` (`GameplayStatics.GetPlayerPawn` 0))
      ;[1 1 1] 控制新角色并重新设置控制器朝向
      (`self.Possess` _returnvalue_3)
      (`self.SetInitialLocationAndRotation` (`self.K2_GetActorLocation` (`GameplayStatics.GetPlayerPawn` 0)) (`self.DefaultRotation`)))))

(fn `UserConstructionScript`)