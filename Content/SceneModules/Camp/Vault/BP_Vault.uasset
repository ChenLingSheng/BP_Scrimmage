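; BP_Vault is a camp's destructible vault whose loss ends the vault-defend match.
; BeginPlay caches its UMG_EnergyBlock_HP widget instance so health changes reach the on-actor HP bar.
; AnyDamage feeds a hurt event, named as a server multicast, that lowers HP, refreshes the bar and destroys the actor at zero.
; EndPlay reports CampIndex to GS_VaultDefend's game-over event, whatever the reason the actor ends.
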(event `self.ReceiveBeginPlay`
  ;[1 1 1] 为UMG类指定该类的实例化对象（不进行指定会出现数据与实例化HP血条UI无法联动的情况）
  (bind _asumg_energy_block_hp (cast `/Game/UMGs/UMG_Characters/UMG_EnergyBlock_HP` (`WidgetComponent.GetUserWidgetObject` (`self.Widget`))))
  (set `self.As UMG Energy Block HP` _asumg_energy_block_hp)
  (`self.Upadte HP UI`))

(event `EVE_In_Server_Multicast_ReceiveHurt`
  ;[1 1 1] 接收伤害
  (bind _output_get (set `self.CurrentHP` (- (`self.CurrentHP`) (stale `self.ReceiveAnyDamage` Damage))))
  (if (<= _output_get 0.0)
    (set `self.CurrentHP` 0.0)
    (`self.Upadte HP UI`)
    (`self.K2_DestroyActor`)
    (else
      (`self.Upadte HP UI`))))

(event `self.ReceiveAnyDamage`
  (params (Damage :type "Float (single-precision)") (DamageType :type "DamageType Object Reference") (InstigatedBy :type "Controller Object Reference") (DamageCauser :type "Actor Object Reference"))
  ;[1 1 1] 接收伤害
  (`self.EVE_In_Server_Multicast_ReceiveHurt`))

(event `self.ReceiveEndPlay`
  (params (EndPlayReason :type "EEndPlayReason Enum" :default "Destroyed"))
  (bind _asgs_vault_defend (cast `/Game/Maps/Game/VaultDefense/GS_VaultDefend` (`GameplayStatics.GetGameState`)))
  (`/Game/Maps/Game/VaultDefense/GS_VaultDefend.CE_GameOver` _asgs_vault_defend (`self.CampIndex`)))

(fn `Upadte HP UI`
  (`/Game/UMGs/UMG_Characters/UMG_EnergyBlock_HP.Update HP UI` (`self.As UMG Energy Block HP`) (`self.CurrentHP`) (`self.MaxHP`)))

(fn `UserConstructionScript`)