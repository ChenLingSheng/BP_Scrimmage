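; Base pickup item actor that floats in the scene until a hero collects it.
; An autoplaying, looping Floating timeline spins and bobs the StaticMesh, with a random start position on BeginPlay to vary each item's animation.
; Sphere overlap with a BP_Hero_Base calls PickUpItemResult, an empty event here, then stops the animation, zeroes ItemNumber on BPItemBuilder and destroys the actor.
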(event `self.ReceiveBeginPlay`
  ;[1 1 1] 为“Floating”时间轴设置随机播放位置
  (`TimelineComponent.SetPlaybackPosition` (`self.Floating`) (`KismetMathLibrary.RandomFloatInRange` 0.0 5.0) false true))

(event `PickUpItemResult`
  (params (`Other Actor` :type "/Game/Characters/Heros/Base/Blueprint/BP_Hero_Base Object Reference")))

(event `self.Sphere.OnComponentBeginOverlap`
  (params (OverlappedComponent :type "PrimitiveComponent Object Reference") (OtherActor :type "Actor Object Reference") (OtherComp :type "PrimitiveComponent Object Reference") (OtherBodyIndex :type Integer) (bFromSweep :type Boolean) (SweepResult :type "HitResult Structure (by ref)"))
  (bind _asbp_hero_base (cast `/Game/Characters/Heros/Base/Blueprint/BP_Hero_Base` OtherActor))
  (`self.PickUpItemResult` _asbp_hero_base)
  (`TimelineComponent.Stop` (`self.Floating`)) ; 停止浮动动画
  (set `/Game/SceneModules/Item/BP_ItemBuilder.ItemNumber` 0 (`self.BP_ItemBuilder`))
  (`self.K2_DestroyActor`))

(fn `UserConstructionScript`)