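; Shooter hero character Blueprint that implements the hero's normal and skill attacks as ranged shots.
; Each attack disables input, plays its fire montage, requests a bullet of the matching type, and restores input on blend out; the skill first sets the actor's rotation.
; FUN_ServerFire spawns a BP_Fire_Base projectile only with authority, at the weapon socket facing capsule forward, passing camp, damage and bullet type.
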(event `self.ReceiveBeginPlay`
  (`parent.ReceiveBeginPlay`))

(event `self.CE_ExecuteNormalAttak`
  ;[1 1 1] 普通攻击
  (`self.DisableInput` null)
  (`|PlayMontage` (`self.Mesh`) "/Game/Characters/Heros/Shooter/Animations/Fire_B_Montage.Fire_B_Montage"
    (:`then`
      (bind _output_get (set `self.BulletType` "NewEnumerator0"))
      (`self.FUN_ServerFire` _output_get))
    (:`OnBlendOut`
      (`self.EnableInput` null))))

(event `self.CE_ExecuteSkillAttak`
  ;[1 1 1] 技能攻击
  (`self.FUN_SetActorRotation`)
  (`self.DisableInput` null)
  (`|PlayMontage` (`self.Mesh`) "/Game/Characters/Heros/Shooter/Animations/Fire_A_Montage.Fire_A_Montage"
    (:`then`
      (bind _output_get (set `self.BulletType` "NewEnumerator1"))
      (`self.FUN_ServerFire` _output_get))
    (:`OnBlendOut`
      (`self.EnableInput` null))))

(fn `FUN_ServerFire`
  (params (BulletType :type "/Game/Characters/Heros/Shooter/Weapons/Bullet_Ranged/E_BulletType Enum" :default "NewEnumerator0"))
  ;[1 1 1] 只在服务器执行
  (`/Engine/EditorBlueprintResources/ActorMacros.Switch Has Authority`
    (:`Authority`
      (`|SpawnActorFromClass` "/Game/Characters/Heros/Shooter/Weapons/Bullet_Ranged/BP_Fire_Base.BP_Fire_Base_C" (`KismetMathLibrary.MakeTransform` (`SceneComponent.GetSocketLocation` (`self.Mesh`) "WeaponFirePoint") (`KismetMathLibrary.Conv_VectorToRotator` (`SceneComponent.GetForwardVector` (`self.CapsuleComponent`)))) "Undefined" "OverrideRootScale" null (`self.Player Camp Index`) (`self.CurrentDamage`) BulletType null))))

(fn `UserConstructionScript`
  (`parent.UserConstructionScript`))