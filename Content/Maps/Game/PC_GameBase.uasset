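; Base game player controller that handles hero spawning, death, timed revival and leaving the session to the login level.
; On local BeginPlay it spawns and possesses a hero using GameInstance choices and data tables for class and camp start.
; It polls with short delays until pawn and hero are valid to set initial rotation.
; Death swaps possession to a camera pawn and shows a countdown before spawning a fresh hero.
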(event `self.ReceiveBeginPlay`
  (bind _returnvalue (`GameplayStatics.GetPlayerPawn` 0))
  (bind _bp_hero (`self.BP_Hero`))
  (bind _returnvalue_2 (`self.K2_GetActorRotation` _returnvalue))
  ;[1 1 1] 生成Pawn并控制
  ;;[1 1 1] 只在本地执行
  (if (`self.IsLocalPlayerController`)
    (`|ExecutionSequence`
      (:`then_0`
        (`self.CE_CallSpawnPlayer`)
        ;[1 1 1] 根据 Pawn 的初始朝向设置控制器转向
        (`/Engine/EditorBlueprintResources/StandardMacros.IsValid` _returnvalue :!label _label
          (:`Is Valid`
            (`self.SetInitialLocationAndRotation` (`self.K2_GetActorLocation` _returnvalue) _returnvalue_2)
            (bind _output_get (set `self.DefaultRotation` _returnvalue_2))
            (`/Engine/EditorBlueprintResources/StandardMacros.IsValid` _bp_hero :!label _label_2
              (:`Is Valid`
                (set `/Game/Characters/Heros/Base/Blueprint/BP_Hero_Base.DefaultRotation` _output_get _bp_hero))
              (:`Is Not Valid`
                (`KismetSystemLibrary.Delay` 0.1)
                (goto _label_2))))
          (:`Is Not Valid`
            (`KismetSystemLibrary.Delay` 0.1)
            (goto _label)))))))

(event `CE_CallSpawnPlayer`
  ;[1 1 1] 生成Spawn
  (bind _asgi_main (cast `/Game/GI_Main` (`GameplayStatics.GetGameInstance`)))
  (`self.EVE_Spawn_Player` (`/Game/GI_Main.PlayerName` _asgi_main) (`/Game/GI_Main.PlayerHeroIndex` _asgi_main) (`/Game/GI_Main.PlayerCampIndex` _asgi_main) (`/Game/GI_Main.playerIndexForCamp` _asgi_main)))

(event `EVE_Spawn_Player`
  (params (PlayerName :type Text) (PlayerHeroIndex :type Integer) (PlayerCampIndex :type Integer) (playerIndexForCamp :type Integer))
  ;[1 1 1] 根据索引生成指定的玩家角色
  (`self.Spawn_Player_Character` PlayerName PlayerHeroIndex PlayerCampIndex playerIndexForCamp))

(event `CE_HeroDeath`
  (params (SpawnTransform :type "Transform Structure"))
  ;[1 1 1] 玩家死亡，将本地玩家控制器的Pawn更换为 BP_HeroDeath【在BP_Hero_Base调用】
  (if (`self.IsLocalPlayerController`)
    (`self.CE_Spawn_BP_DeathCamera` SpawnTransform)
    (`self.Create_UMG_ReviveTimer`)
    (`KismetSystemLibrary.K2_SetTimerDelegate` (delegate `Revive Hero`) (`KismetMathLibrary.Conv_IntToDouble` (`self.ReviveTime`)))))

(event `Revive Hero`
  (bind _bp_herodeath (`self.BP_HeroDeath`))
  ;[1 1 1] 复活（重新创建一个全新的Pawn）
  (`self.CE_CallSpawnPlayer`)
  (`/Engine/EditorBlueprintResources/StandardMacros.IsValid` _bp_herodeath
    (:`Is Valid`
      (`self.K2_DestroyActor` _bp_herodeath))))

(event `CE_Spawn_BP_DeathCamera`
  (params (SpawnTransform :type "Transform Structure"))
  ;[1 1 1] 在服务端上生成 BP_DeathCamera 并让对应的客户端 PlayerController 获取控制权
  (bind _returnvalue (`|SpawnActorFromClass` "/Game/Characters/Heros/BP_Death_Camera.BP_Death_Camera_C" SpawnTransform "Undefined" "OverrideRootScale" null null))
  (set `self.BP_HeroDeath` _returnvalue)
  (`self.Possess` _returnvalue))

(event `CE_Client_Quit_Session`
  ;[1 1 1] 退出房间
  (`DestroySessionCallbackProxy.DestroySession` self
    (:`OnSuccess`
      (`GameplayStatics.OpenLevelBySoftObjectPtr` "/Game/Maps/Login/L_Login.L_Login"))))

(fn `ConfirmPlayerStart`
  (params (PlayerCampIndex :type Integer) (playerIndex :type Integer))
  (returns (BP_PlayerStart :type "/Game/Maps/Game/BP_PlayerStartBase Object Reference"))
  (bind _returnvalue (`|GetDataTableRow` "/Game/Maps/Game/DT_PlayerStart.DT_PlayerStart" (`|GetArrayItem` (`self.PlayerCampNames`) PlayerCampIndex))
    (:`then`
      (bind _outactors (`GameplayStatics.GetAllActorsOfClass` (`.PlayerStart_3_554C793141EA6F0BFA077BACB520F902` (break `/Game/Maps/Game/F_PlayerStart` _returnvalue))))
      (return (`|GetArrayItem` _outactors playerIndex)))))

(fn `Create_UMG_ReviveTimer`
  (bind _returnvalue (`|CreateWidget` "/Game/UMGs/UMG_ReviveTimer.UMG_ReviveTimer_C"))
  (set `/Game/UMGs/UMG_ReviveTimer.Time` (`self.ReviveTime`) _returnvalue)
  (`/Game/UMGs/UMG_ReviveTimer.BeginReviveByTime` _returnvalue)
  (`UserWidget.AddToViewport` _returnvalue 0))

(fn `Spawn_Player_Character`
  (params (PlayerName :type Text) (HeroTypeIndex :type Integer) (PlayerCampIndex :type Integer) (playerIndexForCamp :type Integer))
  (bind (_returnvalue_year _returnvalue_month _returnvalue_day _returnvalue_hour _returnvalue_minute _returnvalue_second _returnvalue_millisecond) (`KismetMathLibrary.BreakDateTime` (`KismetMathLibrary.Now`)))
  (bind _bp_playerstart (`self.ConfirmPlayerStart` PlayerCampIndex playerIndexForCamp))
  (bind _returnvalue (`|GetDataTableRow` "/Game/Characters/Heros/DT_HeroAttribute.DT_HeroAttribute" (`|GetArrayItem` (`self.HeroNames`) HeroTypeIndex))
    (:`then`
      (bind _output_get (set `self.PlayerID` (`KismetStringLibrary.Concat_StrStr` (`KismetStringLibrary.Conv_IntToString` _returnvalue_year) (`KismetStringLibrary.Conv_IntToString` _returnvalue_month) (`KismetStringLibrary.Conv_IntToString` _returnvalue_day) (`KismetStringLibrary.Conv_IntToString` _returnvalue_hour) (`KismetStringLibrary.Conv_IntToString` _returnvalue_minute) (`KismetStringLibrary.Conv_IntToString` _returnvalue_second) (`KismetStringLibrary.Conv_IntToString` _returnvalue_millisecond))))
      (bind _returnvalue_2 (`|SpawnActorFromClass` (`.HeroType_2_F41A0DA2484FBBF976B9B98DCF4E3E16` (break `/Game/Characters/Heros/F_HeroAttribute` _returnvalue)) (`self.GetTransform` _bp_playerstart) "Undefined" "OverrideRootScale" null PlayerName _output_get PlayerCampIndex null))
      (set `self.BP_Hero` _returnvalue_2)
      (`self.Possess` _returnvalue_2)
      (`WidgetBlueprintLibrary.SetInputMode_GameOnly` self))))

(fn `UserConstructionScript`
  (bind _outrownames (`DataTableFunctionLibrary.GetDataTableRowNames` "/Game/Characters/Heros/DT_HeroAttribute.DT_HeroAttribute"))
  (set `self.HeroNames` _outrownames)
  (bind _outrownames_2 (`DataTableFunctionLibrary.GetDataTableRowNames` "/Game/Maps/Game/DT_PlayerStart.DT_PlayerStart"))
  (set `self.PlayerCampNames` _outrownames_2))