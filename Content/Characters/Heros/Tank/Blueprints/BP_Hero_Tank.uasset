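; Tank hero Blueprint that extends a parent hero with its attacks, unique skill and hit reaction.
; The skill briefly doubles walk speed and opens a timed window where the attack plays a different, double-damage montage with input disabled.
; Normal and skill hit events run forward sphere traces into a shared damage check, with the skill's wider, longer trace lifting the returned target upward.
; Received damage restores 1% of its value as energy.
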(event `self.ReceiveActorBeginOverlap`
  (params (OtherActor :type "Actor Object Reference"))
  (`parent.ReceiveActorBeginOverlap` OtherActor))

(event `self.ReceiveTick`
  (params (DeltaSeconds :type "Float (single-precision)"))
  (`parent.ReceiveTick` DeltaSeconds))

(event `self.ReceiveBeginPlay`
  (`parent.ReceiveBeginPlay`))

(event `self.CE_ExecuteNormalAttak`
  ;[1 1 1] Attack
  (`self.DisableInput` null)
  (if (`self.B_Is Unique Skill`)
    (set `self.CurrentDamage` (* 2 (`.DefaultDamge_19_FEFDC9F547540E607FBA77B1D193316C` (break `/Game/Characters/Heros/F_HeroAttribute` (`self.HeroAttribute`)))))
    (`|PlayMontage` (`self.Mesh`) "/Game/Characters/Heros/Tank/Animations/Attack_G_Dusk_Montage.Attack_G_Dusk_Montage"
      (:`OnBlendOut`
        (set `self.CurrentDamage` (`.DefaultDamge_19_FEFDC9F547540E607FBA77B1D193316C` (break `/Game/Characters/Heros/F_HeroAttribute` (`self.HeroAttribute`))))
        (`self.EnableInput` null)
        (set `self.B_Is Unique Skill` false)))
    (else
      (`|PlayMontage` (`self.Mesh`) "/Game/Characters/Heros/Tank/Animations/Attack_A_Montage.Attack_A_Montage"
        (:`OnCompleted`
          (`self.EnableInput` null))))))

(event `self.CE_ExecuteSkillAttak`
  ;[1 1 1] UniqueSkill
  (set `self.B_Is Unique Skill` true)
  (set `CharacterMovementComponent.MaxWalkSpeed` (* 2 (`.MaxWalkSpeed_15_0950319B48614EF6C0FA70A90CEF7DB9` (break `/Game/Characters/Heros/F_HeroAttribute` (`self.HeroAttribute`)))) (`self.CharacterMovement`))
  (`KismetSystemLibrary.K2_SetTimerDelegate` (delegate `CE_SetWalkSpeed`) 1.0)
  (`KismetSystemLibrary.K2_SetTimerDelegate` (delegate `CE_Set_B_IsUniqueSkill`) 3.0))

(event `CE_SetWalkSpeed`
  ;[1 1 1] UniqueSkill
  (set `CharacterMovementComponent.MaxWalkSpeed` (`.MaxWalkSpeed_15_0950319B48614EF6C0FA70A90CEF7DB9` (break `/Game/Characters/Heros/F_HeroAttribute` (`self.HeroAttribute`))) (`self.CharacterMovement`)))

(event `CE_Set_B_IsUniqueSkill`
  ;[1 1 1] UniqueSkill
  (set `self.B_Is Unique Skill` false))

(event `self.CE_MakeNormalHurt`
  ;[1 1 1] 检测普通攻击对象并应用伤害
  (bind (_outhits _returnvalue) (`self.FUN_Forward_MultiSpereTraceForObjects` 80.0 90.0 150.0 self))
  (`self.FUN_DetectionAttackTarget` _outhits _returnvalue))

(event `self.CE_MakeSkillHurt`
  ;[1 1 1] 检测技能攻击对象并应用伤害
  (bind (_outhits _returnvalue) (`self.FUN_Forward_MultiSpereTraceForObjects` 100.0 90.0 200.0 self))
  (bind _hitactor (`self.FUN_DetectionAttackTarget` _outhits _returnvalue))
  (`/Engine/EditorBlueprintResources/StandardMacros.IsValid` _hitactor
    (:`Is Valid`
      (`self.K2_AddActorWorldOffset` _hitactor (0.0 0.0 300.0) false false))))

(event `self.CE_ReceiveHurtPlus`
  (params (`Receive Hurt Value` :type "Float (single-precision)"))
  ;[1 1 1] 角色受击特定事件（按接收的伤害的1%恢复能量值）
  (set `self.CurrentEnergy` (+ (/ `Receive Hurt Value` 100.0) (`self.CurrentEnergy`))))

(fn `UserConstructionScript`
  (`parent.UserConstructionScript`))