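; Player controller for the VaultDefense game mode that manages the local match timer and game-over screens.
; On begin play the local controller creates and starts the timer widget, and a custom event writes game time into GS_VaultDefend.
; The game-over event stores the winner, freezes play via zero time dilation and pause, then shows the result widget locally with UI-only input.
; An unconnected branch would reset player data in GI_Main.
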(event `self.ReceiveBeginPlay`
  (`parent.ReceiveBeginPlay`)
  (if (`self.IsLocalPlayerController`)
    (`self.FUN_Create_UMG_GameTimer`)))

(event `CE_Update_GameTime`
  (params (GameTime :type Text))
  (bind _asgs_vault_defend (cast `/Game/Maps/Game/VaultDefense/GS_VaultDefend` (`GameplayStatics.GetGameState`)))
  (set `/Game/Maps/Game/VaultDefense/GS_VaultDefend.GameTime` GameTime _asgs_vault_defend))

(event `CE_Spawn_UMG_GameOver`
  (params (`Winning Player Name` :type Text))
  (bind _returnvalue (`GameplayStatics.GetPlayerController` 0))
  (set `self.Winning Player Name` `Winning Player Name`)
  (`self.FUN_SetGameStop`)
  (if (`self.IsLocalPlayerController`)
    (`self.FUN_Create_UMG_GameOver`)
    (set `PlayerController.bShowMouseCursor` true _returnvalue)
    (`WidgetBlueprintLibrary.SetInputMode_UIOnlyEx` _returnvalue null)))

(fn `FUN_Create_UMG_GameOver`
  (bind _returnvalue (`|CreateWidget` "/Game/UMGs/UMG_GameOver.UMG_GameOver_C"))
  (`/Engine/EditorBlueprintResources/StandardMacros.IsValid` _returnvalue
    (:`Is Valid`
      (bind _output_get (set `self.UMG_GameOver` _returnvalue))
      (`/Game/UMGs/UMG_GameOver.Set Winning Player Name` _output_get (`self.Winning Player Name`))
      (set `/Game/UMGs/UMG_GameOver.PlayerID` (`self.PlayerID`) (`self.UMG_GameOver`))
      (`UserWidget.AddToViewport` (`self.UMG_GameOver`) 0))))

(fn `FUN_Create_UMG_GameTimer`
  (bind _returnvalue (`|CreateWidget` "/Game/UMGs/UMG_GameTimer.UMG_GameTimer_C"))
  (bind _output_get (set `self.UMG_GameTimer` _returnvalue))
  (`/Game/UMGs/UMG_GameTimer.EVE_StartUseGameTimer` _output_get)
  (`UserWidget.AddToViewport` _output_get 0))

(fn `FUN_SetGameStop`
  (`GameplayStatics.SetGlobalTimeDilation` 0.0)
  (`GameplayStatics.SetGamePaused` true))

(fn `UserConstructionScript`
  (`parent.UserConstructionScript`))