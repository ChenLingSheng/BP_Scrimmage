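; Fire base actor for the Shooter hero's ranged weapon that spawns a fan of bullets from its own transform.
; The construction script loads the DT_BulletAttribute row matching its BulletType enum.
; On BeginPlay, authority only, it spawns the row's bullet class in yaw steps of SectorAngle / BulletCount from minus half the sector, passing damage and camp index.
; It then plays audio, destroying itself only if an immediate play-state check returns FadingOut.
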(event `self.ReceiveBeginPlay`
  ;[1 1 1] 只在客户端执行
  (`/Engine/EditorBlueprintResources/ActorMacros.Switch Has Authority`
    (:`Authority`
      (`self.SetBulletTypeAndSpawnBullet`))))

(fn `SetBulletTypeAndSpawnBullet`
  (locals (SectorAngleSplit :type "Float (double-precision)") (Location :type "Vector Structure") (Rotation :type "Rotator Structure"))
  (bind _audio (`self.Audio`))
  (bind ((`BulletCount_9_A7E6318C4CD6A7920E08C1A550FD75BB` _bulletcount) (`SectorAngle_12_85D91CD540D077B0C70C548191D1E88D` _sectorangle)) (break `/Game/Characters/Heros/Shooter/Weapons/Bullet_Ranged/F_BulletAttribute` (`self.F_BulletAttribute`)))
  ;[1 1 1] 设置子弹间隔角度、子弹生成 Location 、第一颗子弹的 Rotation
  (set `local.SectorAngleSplit` (/ _sectorangle (`KismetMathLibrary.Conv_IntToDouble` _bulletcount)))
  (set `local.Location` (`self.K2_GetActorLocation` self))
  (set `local.Rotation` (`self.K2_GetActorRotation` self))
  (set `local.Rotation` (`KismetMathLibrary.MakeRotator` (.roll (`local.Rotation`)) (.pitch (`local.Rotation`)) (- (.yaw (`local.Rotation`)) (/ _sectorangle 2.0))))
  ;[1 1 1] 根据 Bullet Attribute 循环生成全部子弹
  (for _ (range 1 (+ (`.BulletCount_9_A7E6318C4CD6A7920E08C1A550FD75BB` (break `/Game/Characters/Heros/Shooter/Weapons/Bullet_Ranged/F_BulletAttribute` (`self.F_BulletAttribute`))) 1))
    (`|SpawnActorFromClass` (`.BulletType_3_37F55EAC41D32AA0CDF8729AFDAB9FA6` (break `/Game/Characters/Heros/Shooter/Weapons/Bullet_Ranged/F_BulletAttribute` (`self.F_BulletAttribute`))) (`KismetMathLibrary.MakeTransform` (`local.Location`) (`local.Rotation`)) "Undefined" "OverrideRootScale" null (`self.DamageValue`) (`self.PlayerCampIndex`) null)
    ;[1 1 1] 在上一颗子弹的 Rotation 基础上加上间隔角度
    (set `local.Rotation` (`KismetMathLibrary.MakeRotator` (.roll (`local.Rotation`)) (.pitch (`local.Rotation`)) (+ (.yaw (`local.Rotation`)) (`local.SectorAngleSplit`)))))
  ;[1 1 1] 完成子弹生成后，播放音频，然后销毁自身
  (`AudioComponent.Play` _audio 0.0)
  (if (`|EnumEquality` (`AudioComponent.GetPlayState` _audio) "FadingOut")
    (`self.K2_DestroyActor`)))

(fn `UserConstructionScript`
  (bind _returnvalue (`|GetEnumeratorNameAsString` (`self.BulletType`)))
  ;[1 1 1] 根据需要生成的 Bullet Type 获取到对应的结构体
  (bind _outrownames (`DataTableFunctionLibrary.GetDataTableRowNames` "/Game/Characters/Heros/Shooter/Weapons/Bullet_Ranged/DT_BulletAttribute.DT_BulletAttribute"))
  (for _array_element _outrownames
    (if (== _array_element (`KismetStringLibrary.Conv_StringToName` _returnvalue))
      (bind _returnvalue_2 (`|GetDataTableRow` "/Game/Characters/Heros/Shooter/Weapons/Bullet_Ranged/DT_BulletAttribute.DT_BulletAttribute" (`KismetStringLibrary.Conv_StringToName` _returnvalue))
        (:`then`
          (set `self.F_BulletAttribute` _returnvalue_2)
          (break))))))