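; GM_GameBase is the base game mode for in-game maps, tracking the player controllers of connected players.
; PostLogin adds each PC_GameBase to PCList without duplicates, and OnLogout removes it when the player leaves.
; FUN_Find_PC_ByID looks up a controller by comparing a given PlayerID against the PlayerID on each controller's possessed BP_Hero_Base pawn.
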(event `self.ReceiveBeginPlay`)

(event `self.K2_PostLogin`
  (params (NewPlayer :type "PlayerController Object Reference"))
  ;[1 1 1] 玩家加入：将进入大厅的新玩家的控制器添加到数组中
  (bind _aspc_game_base (cast `/Game/Maps/Game/PC_GameBase` NewPlayer))
  (bind _returnvalue (`KismetArrayLibrary.Array_AddUnique` (`self.PC_List`) _aspc_game_base))
  (set `self.PC_ListIndex` _returnvalue))

(event `self.K2_OnLogout`
  (params (ExitingController :type "Controller Object Reference"))
  ;[1 1 1] 玩家退出：将退出大厅的玩家的控制器从数组中移除
  (bind _aspc_game_base (cast `/Game/Maps/Game/PC_GameBase` ExitingController))
  (`KismetArrayLibrary.Array_RemoveItem` (`self.PC_List`) _aspc_game_base))

(fn `FUN_Find_PC_ByID`
  (params (PlayerID :type String))
  (returns (PC :type "/Game/Maps/Game/PC_GameBase Object Reference"))
  (for _array_element (`self.PC_List`)
    (bind _asbp_hero_base (cast `/Game/Characters/Heros/Base/Blueprint/BP_Hero_Base` (`Controller.K2_GetPawn` _array_element)))
    (if (`KismetStringLibrary.EqualEqual_StrStr` (`/Game/Characters/Heros/Base/Blueprint/BP_Hero_Base.Player ID` _asbp_hero_base) PlayerID)
      (return _array_element))))

(fn `UserConstructionScript`)